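; BP_MasterRoom is a procedural dungeon room, apparently a base class, that provides enemy spawning and door control.
; SpawnEnemy spawns a given class at a given transform and records the actor in SpawnedObjects.
; CloseDoors and OpenDoors toggle visibility and collision on static mesh children of the ClosedDoors component.
; The event graph and construction script are empty, so nothing here triggers these functions.
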(event EventBeginPlay)

(event Collision|EventActorBeginOverlap
  (params (OtherActor :type Actor%20Object%20Reference)))

(event EventTick
  (params (DeltaSeconds :type Float%20%28single-precision%29)))

(fn ConstructionScript)

(fn SpawnEnemy
  (params (Class :type Actor%20Class%20Reference) (SpawnTransform :type Transform))
  (bind _returnvalue (Game|SpawnActorfromClass Class SpawnTransform "Undefined" "MultiplyWithRoot" 0 0))
  (Utilities|Array|Add (Variables|Default|GetSpawnedObjects) _returnvalue))

(fn CloseDoors
  (bind _closeddoors (Variables|Default|GetClosedDoors))
  (bind _children (Components|GetChildrenComponents _closeddoors false))
  (if (Utilities|Array|IsNotEmpty _children)
    (for _array_element _children
      (bind _asstatic_mesh_component (Utilities|Casting|CastToStaticMeshComponent _array_element))
      (Rendering|SetVisibility _asstatic_mesh_component true false)
      (Collision|SetCollisionEnabled _asstatic_mesh_component "QueryAndPhysics"))))

(fn OpenDoors
  (bind _closeddoors (Variables|Default|GetClosedDoors))
  (bind _children (Components|GetChildrenComponents _closeddoors false))
  (if (Utilities|Array|IsNotEmpty _children)
    (for _array_element _children
      (bind _asstatic_mesh_component (Utilities|Casting|CastToStaticMeshComponent _array_element))
      (Rendering|SetVisibility _asstatic_mesh_component false false)
      (Collision|SetCollisionEnabled _asstatic_mesh_component "NoCollision"))))