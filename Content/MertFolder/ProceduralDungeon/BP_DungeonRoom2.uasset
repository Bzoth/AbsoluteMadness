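; BP_DungeonRoom2 is a procedural dungeon room that locks the player into a combat encounter with two waves of enemies.
; When the player first enters its trigger box, it closes the doors and spawns two BP_AnimeGirl enemies at fixed transforms.
; A looping timer prunes destroyed enemies from SpawnedObjects, spawning two skeletons when the list first empties and reopening the doors when it empties again.
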(event OnComponentBeginOverlap(Box)
  (params (OverlappedComponent :type Primitive%20Component%20Object%20Reference) (OtherActor :type Actor%20Object%20Reference) (OtherComp :type Primitive%20Component%20Object%20Reference) (OtherBodyIndex :type Integer) (bFromSweep :type Boolean) (SweepResult :type Hit%20Result%20Structure%20%28by%20ref%29))
  (if (and (Actor|ActorHasTag OtherActor "Player") (== (Variables|Default|GetisEntered) false))
    (Variables|Default|SetisEntered true)
    (CallFunction|CloseDoors)
    (CallFunction|SpawnEnemy "/Game/MertFolder/Blueprint/BP_AnimeGirl.BP_AnimeGirl_C" (Transformation|GetWorldTransform (Variables|Default|GetSpawnTransform1)))
    (CallFunction|SpawnEnemy "/Game/MertFolder/Blueprint/BP_AnimeGirl.BP_AnimeGirl_C" (Transformation|GetWorldTransform (Variables|Default|GetSpawnTransform2)))
    (CallFunction|StartTimer)))

(event Custom|CheckRoomFinished
  (for _array_element (Variables|Default|GetSpawnedObjects)
    (Utilities|IsValid _array_element
      (:Is%20Not%20Valid
        (Utilities|Array|RemoveItem (Variables|Default|GetSpawnedObjects) _array_element))))
  (if (Utilities|Array|IsEmpty (Variables|Default|GetSpawnedObjects))
    (if (== (Variables|Default|GetVawe) 1)
      (CallFunction|OpenDoors)
      (else
        (Math|Integer|IncrementInt (Variables|Default|GetVawe)
          (:%20%20
            (CallFunction|SpawnEnemy "/Game/MertFolder/Blueprint/BP_Skeleton.BP_Skeleton_C" (Transformation|GetWorldTransform (Variables|Default|GetSpawnTransform1)))
            (CallFunction|SpawnEnemy "/Game/MertFolder/Blueprint/BP_Skeleton.BP_Skeleton_C" (Transformation|GetWorldTransform (Variables|Default|GetSpawnTransform2)))))))))

(event Custom|StartTimer
  (Utilities|Time|SetTimerbyEvent (delegate Custom|CheckRoomFinished) 5.0 true))

(event EventBeginPlay
  (|CallParentFunction)
  (CallFunction|OpenDoors))

(fn ConstructionScript
  (|CallParentFunction))