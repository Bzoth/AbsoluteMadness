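; Procedural dungeon generator that spawns a start room at BeginPlay, then attaches random rooms to open exits using a seeded stream.
; The seed is saved and reloaded, or regenerated when no save exists or the game instance requests one.
; Overlapping rooms are destroyed and retried under a DoN cap on total attempts, while valid rooms add their exits.
; Reaching MaxRoomCount sets leftover exits' child meshes to walls.
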(event Custom|StartSpawnRoom
  (bind _returnvalue (Game|SpawnActorfromClass "/Game/MertFolder/ProceduralDungeon/BP_StartDungeonRoom.BP_StartDungeonRoom_C" (Transformation|GetWorldTransform (Variables|Default|GetDefaultSceneRoot)) "AlwaysSpawn" "MultiplyWithRoot" 0 0))
  (Utilities|Array|AppendArray (Variables|Default|GetExitsList) (Components|GetChildrenComponents (Variables|/Game/MertFolder/ProceduralDungeon/BP_MasterRoom.BP_MasterRoom_C|GetExits _returnvalue) false)))

(event Custom|Spawn%20Next%20Room
  (Utilities|FlowControl|DoN 16
    (:Exit
      (bind _output_get (Variables|Default|SetSelectedExit (.OutItem (Utilities|Array|RandomFromStream (Variables|Default|GetExitsList) (Variables|Default|GetStream)))))
      (bind _returnvalue (Game|SpawnActorfromClass (.OutItem (Utilities|Array|RandomFromStream (Variables|Default|GetDungeonRoomsList) (Variables|Default|GetStream))) (Transformation|GetWorldTransform _output_get) "Undefined" "MultiplyWithRoot" 0 0))
      (bind _asbp_master_room (Utilities|Casting|CastToBP_MasterRoom _returnvalue))
      (Variables|Default|SetLatestRoom _asbp_master_room)
      (CallFunction|CheckforOverlap))))

(event Custom|AddOverlapingRoomsToTheList
  (for _array_element (Components|GetChildrenComponents (Variables|/Game/MertFolder/ProceduralDungeon/BP_MasterRoom.BP_MasterRoom_C|GetCollisions (Variables|Default|GetLatestRoom)) false)
    (bind _asbox_collision (Utilities|Casting|CastToBoxComponent _array_element))
    (Utilities|Array|AppendArray (Variables|Default|GetOverlapingRoomsList) (Class|PrimitiveComponent|GetOverlappingComponents _asbox_collision))))

(event Custom|CheckForOverlap
  (CallFunction|AddOverlapingRoomstotheList)
  (if (Utilities|Array|IsNotEmpty (Variables|Default|GetOverlapingRoomsList))
    (Utilities|Array|Clear (Variables|Default|GetOverlapingRoomsList))
    (Actor|DestroyActor (Variables|Default|GetLatestRoom))
    (CallFunction|SpawnNextRoom)
    (else
      (Utilities|Array|Clear (Variables|Default|GetOverlapingRoomsList))
      (Math|Integer|IncrementInt (Variables|Default|GetCurrentRoomCount)
        (:%20%20
          (Utilities|Array|RemoveItem (Variables|Default|GetExitsList) (Variables|Default|GetSelectedExit))
          (Utilities|Array|AppendArray (Variables|Default|GetExitsList) (Components|GetChildrenComponents (Variables|/Game/MertFolder/ProceduralDungeon/BP_MasterRoom.BP_MasterRoom_C|GetExits (Variables|Default|GetLatestRoom)) false))
          (if (!= (Variables|Default|GetCurrentRoomCount) (Variables|Default|GetMaxRoomCount))
            (CallFunction|SpawnNextRoom)
            (else
              (CallFunction|ClosingHoes))))))))

(event Custom|ClosingHoes
  (for _array_element (Variables|Default|GetExitsList)
    (if (Utilities|Array|IsNotEmpty (Components|GetChildrenComponents _array_element false))
      (for _array_element_2 (Components|GetChildrenComponents _array_element false)
        (bind _asstatic_mesh_component (Utilities|Casting|CastToStaticMeshComponent _array_element_2))
        (Components|StaticMesh|SetStaticMesh _asstatic_mesh_component "/Game/LowPolyMedievalConstructions/Meshes/SM_Wall_3B_TwoSided.SM_Wall_3B_TwoSided")))))

(event Custom|Set%20Seed
  (Utilities|FlowControl|DoOnce false
    (:Completed
      (bind _returnvalue (SaveGame|DoesSaveGameExist "save7"))
      (if _returnvalue
        (bind _asgi_game_instance (Utilities|Casting|CastToGI_GameInstance (Game|GetGameInstance)))
        (bind _output_get (Variables|Default|SetAs%20GI%20Game%20Instance _asgi_game_instance))
        (if (Variables|/Game/FirstPerson/YunusMain/Blueprints/Various/GI_GameInstance.GI_GameInstance_C|GetNewSeed _output_get)
          (Variables|/Game/FirstPerson/YunusMain/Blueprints/Various/GI_GameInstance.GI_GameInstance_C|SetNewSeed (Variables|Default|GetAs%20GI%20Game%20Instance) false)
          (bind _returnvalue_2 (SaveGame|CreateSaveGameObject "/Game/FirstPerson/YunusMain/Blueprints/Various/BP_SaveSystem.BP_SaveSystem_C" :!label _label))
          (Class|KismetMathLibrary|SeedRandomStream (Variables|Default|GetStream))
          (bind _output_get_2 (Variables|Default|SetSavedSeed (Class|KismetMathLibrary|BreakRandomStream (Variables|Default|GetStream))))
          (bind _output_get_3 (Variables|/Game/FirstPerson/YunusMain/Blueprints/Various/BP_SaveSystem.BP_SaveSystem_C|SetSavedSeed _returnvalue_2 _output_get_2))
          (Development|PrintString (Utilities|String|ToString(Integer) _output_get_3))
          (SaveGame|SaveGametoSlot _returnvalue_2 "save7")
          (else
            (bind _returnvalue_3 (SaveGame|LoadGamefromSlot "save7"))
            (bind _asbp_save_system (Utilities|Casting|CastToBP_SaveSystem _returnvalue_3))
            (Variables|Default|SetSeed (Variables|/Game/FirstPerson/YunusMain/Blueprints/Various/BP_SaveSystem.BP_SaveSystem_C|GetSavedSeed _asbp_save_system))
            (Math|Random|SetRandomStreamSeed (Variables|Default|GetStream) (Variables|Default|GetSeed))
            (bind _output_get_4 (Variables|Default|SetSavedSeed (Class|KismetMathLibrary|BreakRandomStream (Variables|Default|GetStream))))
            (Development|PrintString (Utilities|String|ToString(Integer) _output_get_4))))
        (else
          (goto _label))))))

(event EventBeginPlay
  (CallFunction|SetSeed)
  (CallFunction|StartSpawnRoom)
  (CallFunction|SpawnNextRoom))

(fn ConstructionScript)

(fn SpawnNewRoomFunc)