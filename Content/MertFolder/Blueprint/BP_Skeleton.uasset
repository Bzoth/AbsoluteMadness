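; BP_Skeleton is a bomb-carrying skeleton character that explodes and damages nearby pawns.
; On BeginPlay it spawns BP_SkeletonBomb and attaches it to the left hand socket.
; Damager subtracts health with a brief invulnerability and slowdown window, then calls Attack when health runs out.
; Attack sphere-traces for pawns, sends them damage, spawns an explosion effect, and destroys both bomb and skeleton.
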(event Custom|Attack
  (bind _returnvalue (Transformation|GetActorLocation))
  (bind _outhits (Collision|MultiSphereTraceForObjects _returnvalue _returnvalue 1.2e+02 (Utilities|Array|MakeArray "ObjectTypeQuery3") false 0 "None"))
  (for _array_element _outhits
    (Class|BPICombat|DamagePlayer(Message) (.HitActor (Collision|BreakHitResult _array_element)) 8e+01))
  (Effects|SpawnEmitteratLocation "/Game/Realistic_Starter_VFX_Pack_Vol2/Particles/Explosion/P_Explosion_Big_C.P_Explosion_Big_C" _returnvalue)
  (Actor|DestroyActor (Variables|Default|GetNewVar))
  (Actor|DestroyActor))

(event Custom|WieldBomb
  (bind _returnvalue (Game|SpawnActorfromClass "/Game/MertFolder/Blueprint/BP_SkeletonBomb.BP_SkeletonBomb_C" (Transformation|GetActorTransform) "Undefined" "MultiplyWithRoot" 0 0))
  (bind _output_get (Variables|Default|SetNewVar _returnvalue))
  (Transformation|AttachComponentToComponent _output_get (Variables|Character|GetMesh) "LeftHandSocket" "SnapToTarget" "SnapToTarget" "SnapToTarget" true)
  (Variables|Default|SetisWieldingBomb true))

(event EventBeginPlay
  (CallFunction|WieldBomb))

(event EventDamager
  (params (Damage :type Integer))
  (if (Variables|Default|GetCanBeDamaged)
    (Variables|Default|SetCanBeDamaged false)
    (bind _output_get (Variables|Default|SetHealth (- (Variables|Default|GetHealth) Damage)))
    (Utilities|FlowControl|Sequence
      (:then_0
        (Variables|/Script/Engine.CharacterMovementComponent|SetMaxWalkSpeed (Variables|Character|GetCharacterMovement) 4e+02)
        (Utilities|FlowControl|Delay 0.5)
        (Variables|/Script/Engine.CharacterMovementComponent|SetMaxWalkSpeed (Variables|Character|GetCharacterMovement) 6e+02)
        (Variables|Default|SetCanBeDamaged true))
      (:then_1
        (if (<= _output_get 0)
          (CallFunction|Attack))))))

(fn ConstructionScript)