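; BP_Dababy is an AI-moved pawn that steers toward surfaces detected by traces from its own meshes.
; A looping one-second timer runs CheckTrace, which calls MakeTrace for four static meshes and issues four AIMoveTo requests in one sequence.
; MakeTrace debug-draws a Visibility sphere trace along world +X, regardless of facing, and returns the hit location only when something is hit.
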(event Custom|CheckTrace
  (Utilities|FlowControl|Sequence
    (:then_0
      (bind _out_hit_location (CallFunction|MakeTrace (Variables|Default|GetStaticMesh3)))
      (AI|AIMoveTo self _out_hit_location 0 5.0 false))
    (:then_1
      (bind _out_hit_location_2 (CallFunction|MakeTrace (Variables|Default|GetStaticMesh2)))
      (AI|AIMoveTo self _out_hit_location_2 0 5.0 false))
    (:then_2
      (bind _out_hit_location_3 (CallFunction|MakeTrace (Variables|Default|GetStaticMesh1)))
      (AI|AIMoveTo self _out_hit_location_3 0 5.0 false))
    (:then_3
      (bind _out_hit_location_4 (CallFunction|MakeTrace (Variables|Default|GetStaticMesh)))
      (AI|AIMoveTo self _out_hit_location_4 0 5.0 false))))

(event EventBeginPlay
  (Utilities|Time|SetTimerbyEvent (delegate Custom|CheckTrace) 1.0 true))

(event EventTick
  (params (DeltaSeconds :type Float%20%28single-precision%29)))

(fn ConstructionScript)

(fn MakeTrace
  (params (Target :type Scene%20Component%20Object%20Reference))
  (bind _returnvalue (Transformation|GetWorldLocation Target))
  (bind (_x _y _z) (Math|Vector|BreakVector _returnvalue))
  (bind (_outhit _returnvalue_2) (Collision|SphereTraceByChannel _returnvalue (Math|Vector|MakeVector (+ _x 1e+03) _y _z) 4.0 "TraceTypeQuery1" false 0 "ForDuration"))
  (if _returnvalue_2
    (return (.location _outhit))))